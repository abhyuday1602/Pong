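; Player controller for a paddle pawn that creates the player HUD and handles input.
; The MoveUp axis moves the controlled pawn along world Y.
; StoreVelocity saves the BP_Paddle's Y velocity as a fraction of max speed on the paddle, flags it as having stored energy, prints a message and swaps its cube material to red.
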(event EventBeginPlay
  (bind _returnvalue (UserInterface|CreateWidget "/Game/Blueprints/BP_PlayerHUD.BP_PlayerHUD_C"))
  (UserInterface|Viewport|AddtoViewport _returnvalue 0))

(event Input|ActionEvents|InputActionStoreVelocity
  (params (Key :type Key%20Structure :default "None"))
  (:Pressed
    (bind _asbp_paddle (Utilities|Casting|CastToBP_Paddle (Pawn|GetControlledPawn)))
    (Variables|/Game/Blueprints/BP_Paddle.BP_Paddle_C|SetVelToStore _asbp_paddle (/ (.y (Transformation|GetVelocity _asbp_paddle)) (Class|MovementComponent|GetMaxSpeed (Variables|/Script/Engine.Character|GetCharacterMovement _asbp_paddle))))
    (Variables|/Game/Blueprints/BP_Paddle.BP_Paddle_C|SetStoredEnergy _asbp_paddle true)
    (Development|PrintString "Stored" true true "(R=0.000000,G=1.000000,B=0.247370,A=1.000000)" 0.0)
    (Rendering|Material|SetMaterial (Variables|/Game/Blueprints/BP_Paddle.BP_Paddle_C|GetCube _asbp_paddle) 0 "/AnimationSharing/AnimSharingRed.AnimSharingRed")))

(event Input|AxisEvents|InputAxisMoveUp
  (params (AxisValue :type Float%20%28single-precision%29))
  (Pawn|Input|AddMovementInput (Pawn|GetControlledPawn) "0.000000,1.000000,0.000000" AxisValue false))

(fn ConstructionScript)