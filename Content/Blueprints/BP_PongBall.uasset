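; Pong ball pawn that starts in a random diagonal direction and moves each tick through FloatingPawnMovement.
; Wall overlaps flip Y; paddle overlaps flip X, add paddle motion or stored energy as Y deflection, multiply max speed, then clear the stored energy and reset the paddle's material.
; Goal overlaps spawn a replacement ball, increment the player or enemy score in BP_GameMode, and destroy this ball.
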(event OnComponentBeginOverlap(Sphere)
  (params (OverlappedComponent :type Primitive%20Component%20Object%20Reference) (OtherActor :type Actor%20Object%20Reference) (OtherComp :type Primitive%20Component%20Object%20Reference) (OtherBodyIndex :type Integer) (bFromSweep :type Boolean) (SweepResult :type Hit%20Result%20Structure%20%28by%20ref%29))
  (bind _floatingpawnmovement (Variables|Default|GetFloatingPawnMovement))
  (Utilities|Casting|CastToBP_Wall OtherActor
    (:then
      (Development|PrintString "wall")
      (Variables|Default|SetVelocity (Math|Vector|MakeVector (.x (Variables|Default|GetVelocity)) (* (.y (Variables|Default|GetVelocity)) -1.0) (.z (Variables|Default|GetVelocity)))))
    (:CastFailed
      (bind _asbp_paddle (Utilities|Casting|CastToBP_Paddle OtherActor)
        (:then
          (Development|PrintString "paddle")
          (Variables|Default|SetVelocity (Math|Vector|MakeVector (* (.x (Variables|Default|GetVelocity)) -1.0) (+ (.y (Variables|Default|GetVelocity)) (select (Variables|/Game/Blueprints/BP_Paddle.BP_Paddle_C|GetStoredEnergy _asbp_paddle) (Variables|/Game/Blueprints/BP_Paddle.BP_Paddle_C|GetVelToStore _asbp_paddle) (/ (.y (Transformation|GetVelocity _asbp_paddle)) (Class|MovementComponent|GetMaxSpeed (Variables|/Script/Engine.Character|GetCharacterMovement _asbp_paddle))))) (.z (Variables|Default|GetVelocity))))
          (Variables|/Script/Engine.FloatingPawnMovement|SetMaxSpeed _floatingpawnmovement (* (Class|MovementComponent|GetMaxSpeed _floatingpawnmovement) (Variables|Default|GetSpeedMultiplier)))
          (Variables|/Game/Blueprints/BP_Paddle.BP_Paddle_C|SetStoredEnergy _asbp_paddle false)
          (Rendering|Material|SetMaterial (Variables|/Game/Blueprints/BP_Paddle.BP_Paddle_C|GetCube _asbp_paddle) 0 "/Engine/BasicShapes/BasicShapeMaterial.BasicShapeMaterial"))
        (:CastFailed
          (bind _asbp_goal (Utilities|Casting|CastToBP_Goal OtherActor))
          (CallFunction|Goal (Variables|/Game/Blueprints/BP_Goal.BP_Goal_C|GetPlayerTargetGoal _asbp_goal))
          (Actor|DestroyActor))))))

(event Custom|Goal
  (params (PlayerGoal? :type Boolean))
  (Game|SpawnActorfromClass "BP_PongBall_C" (Math|Transform|MakeTransform "-30.000000,-120.000000,9.500100") "Undefined" "MultiplyWithRoot" 0 0)
  (bind _asbp_game_mode (Utilities|Casting|CastToBP_GameMode (Game|GetGameMode)))
  (Math|Integer|IncrementInt (select PlayerGoal? (Variables|/Game/Blueprints/BP_GameMode.BP_GameMode_C|GetPlayerScore _asbp_game_mode) (Variables|/Game/Blueprints/BP_GameMode.BP_GameMode_C|GetEnemyScore _asbp_game_mode))
    (:%20%20
      (Actor|DestroyActor))))

(event EventBeginPlay
  (bind _returnvalue (Math|Random|RandomBool))
  (bind _returnvalue_2 (Math|Float|SelectFloat -1.0 1.0 _returnvalue))
  (Variables|Default|SetVelocity (Math|Vector|MakeVector _returnvalue_2 _returnvalue_2 0.0)))

(event EventTick
  (params (DeltaSeconds :type Float%20%28single-precision%29))
  (Class|PawnMovementComponent|AddInputVector (Variables|Default|GetFloatingPawnMovement) (Variables|Default|GetVelocity) false)
  (Development|PrintString (Utilities|String|ToString(Float) (Math|Vector|VectorLength (Transformation|GetVelocity))) true true "(R=0.000000,G=0.660000,B=1.000000,A=1.000000)" 0.0))

(fn ConstructionScript)