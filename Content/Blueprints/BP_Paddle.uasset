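; BP_Paddle is a paddle actor with a CharacterMovement component, confined to a fixed range along the world Y axis.
; Every Tick it checks its location and snaps Y back to a symmetric limit when it passes either edge, leaving X and Z unchanged.
; It also prints its Y velocity as a fraction of max speed each frame as on-screen debug output.
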(event EventTick
  (params (DeltaSeconds :type Float%20%28single-precision%29))
  (bind _returnvalue (Transformation|GetActorLocation))
  (if (> (.y _returnvalue) 3.8e+02)
    (Transformation|SetActorLocation (Math|Vector|MakeVector (.x _returnvalue) 3.8e+02 (.z _returnvalue)) false false)
    (elif (< (.y _returnvalue) -3.8e+02)
      (Transformation|SetActorLocation (Math|Vector|MakeVector (.x _returnvalue) -3.8e+02 (.z _returnvalue)) false false)))
  (Development|PrintString (Utilities|String|ToString(Float) (/ (.y (Transformation|GetVelocity)) (Class|MovementComponent|GetMaxSpeed (Variables|Character|GetCharacterMovement)))) true true "(R=1.000000,G=0.190183,B=0.000000,A=1.000000)" 0.0))

(fn ConstructionScript)