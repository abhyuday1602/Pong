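; BP_EnemyPaddle is the AI opponent paddle in a Pong game, tracking the ball along the Y axis.
; Each Tick it clamps its Y position to a fixed symmetric range by teleporting back to the limit.
; It then looks up BP_PongBall with GetActorOfClass every frame and adds reduced-scale movement input toward the ball's side, always at full direction with no dead zone.
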(event EventBeginPlay)

(event Collision|EventActorBeginOverlap
  (params (OtherActor :type Actor%20Object%20Reference)))

(event EventTick
  (params (DeltaSeconds :type Float%20%28single-precision%29))
  (bind _returnvalue (Transformation|GetActorLocation))
  (if (> (.y _returnvalue) 3.8e+02)
    (Transformation|SetActorLocation (Math|Vector|MakeVector (.x _returnvalue) 3.8e+02 (.z _returnvalue)) false false)
    (elif (< (.y _returnvalue) -3.8e+02)
      (Transformation|SetActorLocation (Math|Vector|MakeVector (.x _returnvalue) -3.8e+02 (.z _returnvalue)) false false)))
  (bind _returnvalue_2 (Actor|GetActorOfClass "/Game/Blueprints/BP_PongBall.BP_PongBall_C"))
  (Pawn|Input|AddMovementInput (Math|Vector|MakeVector 0.0 (Math|Float|SelectFloat 1.0 -1.0 (> (- (.y (Transformation|GetActorLocation _returnvalue_2)) (.y (Transformation|GetActorLocation))) 0.0)) 0.0) 0.7 false))

(fn ConstructionScript
  (|CallParentFunction))